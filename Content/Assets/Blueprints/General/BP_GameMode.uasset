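; BP_GameMode is a game mode Blueprint that handles the start and end screens of a match.
; StartGame creates the start widget for the first player and adds it to the viewport.
; GameOver shows a game-over widget with win or lose text based on its flag, then reopens the Main level after a short delay.
; BeginPlay and Tick are unused, so both events rely on being called.
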(event EventBeginPlay)

(event EventTick
  (params (DeltaSeconds :type Float%20%28single-precision%29)))

(event EventStartGame
  (bind _returnvalue (UserInterface|CreateWidget "/Game/Assets/Blueprints/Widgets/Widget_StartGame.Widget_StartGame_C" (Game|GetPlayerController 0)))
  (UserInterface|Viewport|AddtoViewport _returnvalue 0))

(event EventGameOver
  (params (bWoonGame :type Boolean))
  (bind _returnvalue (UserInterface|CreateWidget "/Game/Assets/Blueprints/Widgets/Widget_GameOver.Widget_GameOver_C"))
  (UserInterface|Viewport|AddtoViewport _returnvalue 0)
  (Rendering|Components|TextRender|SetText (Variables|/Game/Assets/Blueprints/Widgets/Widget_GameOver.Widget_GameOver_C|GetDisplayText _returnvalue) (select bWoonGame "YOU WON!!" "YOU LOST!"))
  (Utilities|FlowControl|Delay 3.0)
  (Game|OpenLevel(byObjectReference) "/Game/Maps/Main.Main"))

(fn ConstructionScript)